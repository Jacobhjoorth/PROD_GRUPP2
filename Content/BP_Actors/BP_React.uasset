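; Overlap-triggered quick-time event actor that makes the player press Spacebar on audio cues, repeated until TotalReacts is reached.
; BeginReact plays start and tension sounds to open each press window, while a self-rescheduling 0.1-second ReactTick timer polls input and checks for timeouts.
; Successes restart the cycle with higher-pitched sounds based on ReactCounter.
; Early or missed presses play a death sound and clear the timer, with outcomes only printed.
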(event Custom|Begin%20React
  (bind _react_start_sfx (Variables|Default|GetReact_Start_SFX))
  ;[0.05729 0.05729 0.05729] Beginplay, enables space press after delay (delay is 0 for now), then another delay for the player to press space to react
  (if (Variables|Default|GetEnable%20Spacebar)
    _
    (else
      (Utilities|FlowControl|Delay 0.0) ; delay b4 space is enabled
    ))
  (Variables|Default|SetEnable%20Spacebar true)
  (Utilities|FlowControl|Delay 1.0) ; delay b4 player should press space
  (bind _pitch_multiplier (CallFunction|IncreasePitch 0.105))
  (Variables|/Script/Engine.AudioComponent|SetPitchMultiplier _react_start_sfx (- _pitch_multiplier 0.14))
  (Audio|Components|Audio|Stop _react_start_sfx)
  (Audio|Components|Audio|Play _react_start_sfx 0.0)
  (Variables|Default|SetShould%20Press%20Spacebar true)
  (Audio|Components|Audio|Play (Variables|Default|GetReact_Tension_SFX) 0.0)
  (Development|PrintString "press space to react"))

(event Custom|React%20Tick
  (bind _react_success_sfx (Variables|Default|GetReact_Success_SFX))
  (bind _react_counter_checker (Variables|Default|GetReact%20Counter%20Checker))
  ;[0.05729 0.05729 0.05729] Checks if player pressed space after space has been enabled
  (bind _returnvalue (Utilities|Time|SetTimerbyEvent (delegate Custom|React%20Tick) 0.1))
  (Variables|Default|SetTimer%20Handle _returnvalue)
  (Utilities|FlowControl|Sequence
    (:then_0
      (if (Game|Player|IsInputKeyDown (Game|GetPlayerController 0) "SpaceBar")
        (if (Variables|Default|GetEnable%20Spacebar)
          (if (Variables|Default|GetShould%20Press%20Spacebar)
            ;[0.05729 0.05729 0.05729] React success
            (Variables|Default|SetEnable%20Spacebar false) ; stops tick
            (Development|PrintString "spacebar successfully pressed")
            (Audio|Components|Audio|Stop (Variables|Default|GetReact_Tension_SFX))
            (bind _pitch_multiplier (CallFunction|IncreasePitch 0.15))
            (Variables|/Script/Engine.AudioComponent|SetPitchMultiplier _react_success_sfx _pitch_multiplier)
            (Audio|Components|Audio|Stop _react_success_sfx)
            (Audio|Components|Audio|Play _react_success_sfx 0.0)
            ;[0.05729 0.05729 0.05729] Calculates how many times to react
            (bind _result (Math|Integer|IncrementInt (Variables|Default|GetReact%20Counter))
              (:%20%20
                (if (== _result (Variables|Default|GetTotal%20Reacts))
                  ;[0.05729 0.05729 0.05729] React finished
                  (Development|PrintString "react successfull")
                  (Utilities|Time|ClearandInvalidateTimerbyHandle (Variables|Default|GetTimer%20Handle))
                  (else
                    ;[0.05729 0.05729 0.05729] React not finished and resets
                    (Utilities|FlowControl|Delay 1.0)
                    (CallFunction|RestartReact)))))
            (else
              ;[0.05729 0.05729 0.05729] Failchecks
              (Development|PrintString "Space pressed too early")
              ;[0.05729 0.05729 0.05729] React failed
              (Variables|Default|SetEnable%20Spacebar false :!label _label) ; stops tick
              (Development|PrintString " failed react")
              (Audio|PlaySound2D "/Game/Audio/Sounds/FX/React_SFX/React_death_SFX.React_death_SFX" (Variables|Default|GetVolume) 1.0 0.0 0 0)
              (Utilities|Time|ClearandInvalidateTimerbyHandle (Variables|Default|GetTimer%20Handle)))))))
    (:then_1
      (if (Variables|Default|GetShould%20Press%20Spacebar)
        (Utilities|FlowControl|Delay (+ (Variables|Default|GetTime%20To%20React) 1.0)) ; time to react
        (if (<= (Variables|Default|GetReact%20Counter) _react_counter_checker)
          (Development|PrintString "spacebar failed to press")
          (goto _label)
          (else
            (Math|Integer|IncrementInt _react_counter_checker)))))))

(event Collision|EventActorBeginOverlap
  (params (OtherActor :type Actor%20Object%20Reference))
  ;[0.05729 0.05729 0.05729] Start react on collision with player
  (Utilities|FlowControl|DoOnce false
    (:Completed
      (CallFunction|BeginReact)
      (CallFunction|ReactTick))))

(fn ConstructionScript)

(fn RestartReact
  (CallFunction|BeginReact)
  (Variables|Default|SetShould%20Press%20Spacebar false))

(fn IncreasePitch
  (params (Multiply%20With :type Float%20%28double-precision%29))
  (return (+ (* (Math|Conversions|ToFloat(Integer) (Variables|Default|GetReact%20Counter)) Multiply%20With) 1.0)))