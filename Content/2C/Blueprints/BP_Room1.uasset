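; BP_Room1 is a room volume that registers its name and sound cue with the level's RoomManager on BeginPlay and shows the name on a text render.
; Ending overlap on its collider clears IsInRoom and notifies the manager.
; Begin overlap only casts to Player; the logic setting IsInRoom true is disconnected.
; Tick uses two DoOnce gates that reset each other to print inside/outside debug messages once per change.
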(event OnComponentBeginOverlap(Collider)
  (params (OverlappedComponent :type Primitive%20Component%20Object%20Reference) (OtherActor :type Actor%20Object%20Reference) (OtherComp :type Primitive%20Component%20Object%20Reference) (OtherBodyIndex :type Integer) (bFromSweep :type Boolean) (SweepResult :type Hit%20Result%20Structure%20%28by%20ref%29))
  ;[1 1 1] Begin/End Overlap
  (Utilities|Casting|CastToPlayer OtherActor))

(event OnComponentEndOverlap(Collider)
  (params (OverlappedComponent :type Primitive%20Component%20Object%20Reference) (OtherActor :type Actor%20Object%20Reference) (OtherComp :type Primitive%20Component%20Object%20Reference) (OtherBodyIndex :type Integer))
  ;[1 1 1] Begin/End Overlap
  (Variables|Default|SetbIsInRoom false)
  (Class|ARoomManager|SetPlayerinRoom (Variables|Default|GetRoomManagerRef) (Variables|Default|GetName) (Variables|Default|GetbIsInRoom)))

(event EventBeginPlay
  ;[1 1 1] Begin Play
  (bind _returnvalue (Actor|GetActorOfClass "/Script/PROD_GRUPP2.ARoomManager"))
  (bind _output_get (Variables|Default|SetRoomManagerRef _returnvalue))
  (Class|ARoomManager|AddRoom _output_get (Variables|Default|GetName) (Variables|Default|GetSoundCue))
  (Rendering|Components|TextRender|SetText (Variables|Default|GetTextRender) (Utilities|Text|ToText(Name) (Variables|Default|GetName))))

(event EventTick
  (params (DeltaSeconds :type Float%20%28single-precision%29))
  ;[1 1 1] Tick
  (if (Variables|Default|GetbIsInRoom)
    (Utilities|FlowControl|DoOnce false :!label _label
      (:Completed
        (Development|PrintString "INSIDE ROOM" true true "(R=0.393497,G=1.000000,B=0.300928,A=1.000000)")
        (goto _label_2 Reset)))
    (else
      (Utilities|FlowControl|DoOnce false :!label _label_2
        (:Completed
          (Development|PrintString "OUTSIDE ROOM" true true "(R=1.000000,G=0.294602,B=0.168740,A=1.000000)")
          (goto _label Reset))))))

(fn ConstructionScript)