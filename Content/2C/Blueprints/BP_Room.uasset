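; BP_Room is a room volume actor that registers a named room and its sound cue with the level's RoomManager.
; On BeginPlay it finds the manager by class, caches it, and adds itself by Name and SoundCue.
; Collider begin and end overlaps report player presence to the manager through SetPlayerInRoom, without checking which actor overlapped.
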(event OnComponentBeginOverlap(Collider)
  (params (OverlappedComponent :type Primitive%20Component%20Object%20Reference) (OtherActor :type Actor%20Object%20Reference) (OtherComp :type Primitive%20Component%20Object%20Reference) (OtherBodyIndex :type Integer) (bFromSweep :type Boolean) (SweepResult :type Hit%20Result%20Structure%20%28by%20ref%29))
  (Class|ARoomManager|SetPlayerinRoom (Variables|Default|GetRoomManagerRef) (Variables|Default|GetName) true))

(event OnComponentEndOverlap(Collider)
  (params (OverlappedComponent :type Primitive%20Component%20Object%20Reference) (OtherActor :type Actor%20Object%20Reference) (OtherComp :type Primitive%20Component%20Object%20Reference) (OtherBodyIndex :type Integer))
  (Class|ARoomManager|SetPlayerinRoom (Variables|Default|GetRoomManagerRef) (Variables|Default|GetName) false))

(event EventBeginPlay
  (bind _returnvalue (Actor|GetActorOfClass "/Script/PROD_GRUPP2.ARoomManager"))
  (bind _output_get (Variables|Default|SetRoomManagerRef _returnvalue))
  (Class|ARoomManager|AddRoom _output_get (Variables|Default|GetName) (Variables|Default|GetSoundCue)))

(event Collision|EventActorBeginOverlap
  (params (OtherActor :type Actor%20Object%20Reference)))

(event EventTick
  (params (DeltaSeconds :type Float%20%28single-precision%29)))

(fn ConstructionScript)