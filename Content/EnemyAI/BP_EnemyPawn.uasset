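; Enemy AI pawn that holds a behaviour state and plays its own audio, with a reset back to its spawn point.
; BeginPlay stores the start transform and default behaviour; ResetEnemy restores behaviour and location (not rotation) and stops the AudioController's current voice line.
; PlaySound swaps clips without restarting one already playing, and StopReact sets both audio volumes to full.
; The player-react overlap, wolf-howl toggles and StopReact binding are disconnected.
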(event OnComponentBeginOverlap(ReactCollider)
  (params (OverlappedComponent :type Primitive%20Component%20Object%20Reference) (OtherActor :type Actor%20Object%20Reference) (OtherComp :type Primitive%20Component%20Object%20Reference) (OtherBodyIndex :type Integer) (bFromSweep :type Boolean) (SweepResult :type Hit%20Result%20Structure%20%28by%20ref%29)))

(event Custom|StopReact
  (Audio|Components|Audio|SetVolumeMultiplier (Variables|Default|GetAudio) 1.0 :!class /Script/Engine.AudioComponent)
  (Audio|Components|Audio|SetVolumeMultiplier (Variables|Default|GetBackgroundSound) 1.0 :!class /Script/Engine.AudioComponent))

(event EventBeginPlay
  (Audio|Components|Audio|Stop (Variables|Default|GetAudio))
  (Variables|AIVariables|SetBehaviour "NewEnumerator0")
  (Variables|Default|SetStart%20Position (Transformation|GetActorLocation))
  (Variables|AIVariables|SetStartRotation (Transformation|GetActorRotation)))

(fn ConstructionScript)

(fn PlaySound
  (params (NewSound :type Sound%20Cue%20Object%20Reference))
  (bind _audio (Variables|Default|GetAudio))
  (bind _returnvalue (Audio|Components|Audio|IsPlaying _audio))
  (Utilities|IsValid NewSound
    (:Is%20Valid
      (if (== NewSound (Variables|/Script/Engine.AudioComponent|GetSound _audio))
        _
        (else
          (Audio|Components|Audio|SetSound _audio NewSound)
          (if _returnvalue
            _
            (else
              _))
          (Audio|Components|Audio|Play _audio 0.0)
          (return))))
    (:Is%20Not%20Valid
      _))
  (if (not _returnvalue)
    (Audio|Components|Audio|Play _audio 0.0)
    (return)))

(fn ResetEnemy
  (Variables|AIVariables|SetBehaviour "NewEnumerator0")
  (bind _returnvalue (Actor|GetActorOfClass "/Script/PROD_GRUPP2.AudioController"))
  (Class|AudioController|StopCurrentVoiceLine _returnvalue)
  (Transformation|SetActorLocation self (Variables|Default|GetStart%20Position) false true))