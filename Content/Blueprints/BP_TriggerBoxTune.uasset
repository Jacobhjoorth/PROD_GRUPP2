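; BP_TriggerBoxTune is a box trigger that tells the Player when it is inside a tune zone.
; Begin and end overlap check the other actor for the "player" tag, then set InTuneTrigger true or false on the Player found through GetActorOfClass.
; Both events print debug strings, and begin overlap resets and increments an InteractCounter that nothing here reads.
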(event OnComponentEndOverlap(Box)
  (params (OverlappedComponent :type Primitive%20Component%20Object%20Reference) (OtherActor :type Actor%20Object%20Reference) (OtherComp :type Primitive%20Component%20Object%20Reference) (OtherBodyIndex :type Integer))
  (Development|PrintString "player left box")
  (if (Actor|ActorHasTag OtherActor "player")
    (bind _returnvalue (Actor|GetActorOfClass "/Game/BP_Actors/Player.Player_C"))
    (Variables|/Game/BP_Actors/Player.Player_C|SetInTuneTrigger _returnvalue false)
    (Development|PrintString "Tune Trigger Is False")))

(event OnComponentBeginOverlap(Box)
  (params (OverlappedComponent :type Primitive%20Component%20Object%20Reference) (OtherActor :type Actor%20Object%20Reference) (OtherComp :type Primitive%20Component%20Object%20Reference) (OtherBodyIndex :type Integer) (bFromSweep :type Boolean) (SweepResult :type Hit%20Result%20Structure%20%28by%20ref%29))
  (bind _output_get (Variables|Default|SetInteractCounter 0))
  (Math|Integer|IncrementInt _output_get
    (:%20%20
      (Development|PrintString "IN BOX")
      (if (Actor|ActorHasTag OtherActor "player")
        (bind _returnvalue (Actor|GetActorOfClass "/Game/BP_Actors/Player.Player_C"))
        (Variables|/Game/BP_Actors/Player.Player_C|SetInTuneTrigger _returnvalue true)
        (Development|PrintString "Tune Trigger Is True")))))

(event EventBeginPlay)

(event EventTick
  (params (DeltaSeconds :type Float%20%28single-precision%29)))

(fn ConstructionScript)