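; Bathroom actor that handles the player's bathroom area and holds audio logic for a wake-up intro.
; OnAudioFinished events chain voice and dragging clips, fade and swap ambience, then re-enable player input.
; The opening sequence that caches Player, disables input and starts the first clip is disconnected.
; IsInBathroom overlaps start the enemy tutorial on entry and toggle wolf howls on exit; NearDoor and spacebar logic are stubs or debug.
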(event OnComponentBeginOverlap(IsInBathroom?)
  (params (OverlappedComponent :type Primitive%20Component%20Object%20Reference) (OtherActor :type Actor%20Object%20Reference) (OtherComp :type Primitive%20Component%20Object%20Reference) (OtherBodyIndex :type Integer) (bFromSweep :type Boolean) (SweepResult :type Hit%20Result%20Structure%20%28by%20ref%29))
  (if (Actor|ActorHasTag OtherActor "player")
    (bind _returnvalue (Actor|GetActorOfClass "/Game/BP_Actors/Player.Player_C"))
    (Variables|/Game/BP_Actors/Player.Player_C|SetIsEnemyTutorial? _returnvalue true)
    (Default|EnemyTutorial _returnvalue)))

(event OnAudioFinished(Waking_Up)
  (Audio|Components|Audio|Play (Variables|Default|GetFindAWay) 0.0)
  (Audio|Components|Audio|Play (Variables|Default|GetAmbience) 0.0)
  (Input|EnableInput (Variables|Default|GetPlayer) (Game|GetPlayerController 0)))

(event OnAudioFinished(1NiceWeMadeIt)
  (Audio|Components|Audio|Play (Variables|Default|GetDragingSound) 0.0)
  (Audio|Components|Audio|FadeOut (Variables|Default|GetAmbience) 4.0 0.0 "Linear" :!class /Script/Engine.AudioComponent)
  (Utilities|FlowControl|Delay 4.0)
  (Audio|Components|Audio|Stop (Variables|Default|GetAmbience))
  (Audio|Components|Audio|SetSound (Variables|Default|GetAmbience) "/Game/Audio/Intro/Bathroom/Bathroom_Ambience.Bathroom_Ambience"))

(event OnAudioFinished(DragingSound)
  (Audio|Components|Audio|Play (Variables|Default|GetWaking_Up) 0.0)
  (Audio|Components|Audio|Play (Variables|Default|GetAmbience) 0.0)
  (Audio|Components|Audio|FadeIn (Variables|Default|GetAmbience) 3.0 0.6 0.0 "Linear" :!class /Script/Engine.AudioComponent))

(event OnComponentBeginOverlap(NearDoor)
  (params (OverlappedComponent :type Primitive%20Component%20Object%20Reference) (OtherActor :type Actor%20Object%20Reference) (OtherComp :type Primitive%20Component%20Object%20Reference) (OtherBodyIndex :type Integer) (bFromSweep :type Boolean) (SweepResult :type Hit%20Result%20Structure%20%28by%20ref%29))
  (if (Actor|ActorHasTag OtherActor "player")
    _))

(event OnComponentEndOverlap(IsInBathroom?)
  (params (OverlappedComponent :type Primitive%20Component%20Object%20Reference) (OtherActor :type Actor%20Object%20Reference) (OtherComp :type Primitive%20Component%20Object%20Reference) (OtherBodyIndex :type Integer))
  (if (Actor|ActorHasTag OtherActor "player")
    (Variables|Default|SetPlayerInBathroom? false)
    (Default|ToggleWolfHowl (Variables|Default|GetPlayer) true)))

(event Custom|Pressed%20spcae
  (Variables|Default|SetPlayerInBathroom? true)
  (if true
    (Development|PrintString "you pressed space")))

(event Input|KeyboardEvents|DebugKeySpaceBar
  (params (Key :type Key%20Structure :default "None") (ActionValue :type Input%20Action%20Value%20Structure))
  (:Pressed
    (Development|PrintString "Hello")
    (CallFunction|PressedSpcae)))

(fn ConstructionScript)