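; Lockpick puzzle actor where the player clears three lock positions in random order; Interact drops the door and destroys the actor.
; Left/right moves the selection, up tests it against the random target, and confirming removes a correct position or resets progress otherwise.
; Tick polls for completion to notify the Player and re-enable wolf howls, and uses paired DoOnce gates to stop audio while the player is in the puzzle trigger.
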(event Custom|Go%20Left%20In%20Puzzel
  (if (Utilities|Enum|Equal(Enum) (Variables|Default|GetCurrentLockEnum) "NewEnumerator0")
    (Audio|PlaySound2D "/Game/Audio/Sounds/FX/LockPickError.LockPickError" 0.3 0.3 0.0 0 0)
    (else
      (Audio|PlaySound2D "/Game/Audio/Cues/LockPickHögerVänster_Cue.LockPickHögerVänster_Cue" 2.0 1.0 0.0 0 0)
      (Development|PrintString "Pressed Left")
      (if (Utilities|Enum|Equal(Enum) (Variables|Default|GetCurrentLockEnum) "NewEnumerator0")
        (Variables|Default|SetCurrentLockEnum "NewEnumerator0")
        (elif (Utilities|Enum|Equal(Enum) (Variables|Default|GetCurrentLockEnum) "NewEnumerator1")
          (Variables|Default|SetCurrentLockEnum "NewEnumerator0")
          (elif (Utilities|Enum|Equal(Enum) (Variables|Default|GetCurrentLockEnum) "NewEnumerator2")
            (Variables|Default|SetCurrentLockEnum "NewEnumerator1")))))))

(event Custom|Go%20Right%20In%20puzzel
  (if (Utilities|Enum|Equal(Enum) (Variables|Default|GetCurrentLockEnum) "NewEnumerator2")
    (Audio|PlaySound2D "/Game/Audio/Sounds/FX/LockPickError.LockPickError" 0.3 0.3 0.0 0 0)
    (else
      (Audio|PlaySound2D "/Game/Audio/Cues/LockPickHögerVänster_Cue.LockPickHögerVänster_Cue" 2.0 1.0 0.0 0 0)
      (Development|PrintString "Pressed Right")
      (if (Utilities|Enum|Equal(Enum) (Variables|Default|GetCurrentLockEnum) "NewEnumerator0")
        (Variables|Default|SetCurrentLockEnum "NewEnumerator1")
        (elif (Utilities|Enum|Equal(Enum) (Variables|Default|GetCurrentLockEnum) "NewEnumerator1")
          (Variables|Default|SetCurrentLockEnum "NewEnumerator2")
          (elif (Utilities|Enum|Equal(Enum) (Variables|Default|GetCurrentLockEnum) "NewEnumerator2")
            (Variables|Default|SetCurrentLockEnum "NewEnumerator2")))))))

(event Custom|Interact%20In%20puzzel
  (if (Variables|Default|GetCorrect)
    (CallFunction|RemovesElementfromArrayifItExists)
    (Variables|Default|SetCorrect false)
    (else
      (Development|PrintString "TRIED TO PRESS SPACE FALSE")
      (CallFunction|ResetLock)
      (Audio|PlaySound2D "/Game/Audio/Cues/LockPickTestFel_Cue.LockPickTestFel_Cue" 0.5 1.0 0.0 0 0))))

(event Custom|Go%20Up%20In%20Puzzle
  (Development|PrintString "Pressed Up")
  (if (Utilities|Enum|Equal(Enum) (Variables|Default|GetCurrentLockEnum) (Variables|Default|GetEnumCounter))
    (Development|PrintString "Rätt")
    (Audio|PlaySound2D "/Game/Audio/Cues/LockPickTestRätt_Cue.LockPickTestRätt_Cue" 1.5 1.0 0.0 0 0)
    (Variables|Default|SetCorrect true)
    (else
      (Development|PrintString "Fel")
      (Audio|PlaySound2D "/Game/Audio/Cues/LockPickTest_Cue.LockPickTest_Cue" 1.5 1.0 0.0 0 0))))

(event Custom|Set%20Counter
  (bind _output_get (Variables|Default|SetEnumCounter (Utilities|Array|Get(acopy) (Variables|Default|GetNotCompletedLocks) (Math|Random|RandomIntegerinRange 0 (Variables|Default|GetMax)))))
  (Development|PrintString (Utilities|String|EnumtoString _output_get) true true "(R=1.000000,G=0.000000,B=0.292559,A=1.000000)" 15.0))

(event EventBeginPlay
  (Variables|Default|SetCurrentLockEnum "NewEnumerator0")
  (CallFunction|SetCounter)
  (bind _returnvalue (Actor|GetActorOfClass "/Game/BP_Actors/Player.Player_C"))
  (Variables|Default|SetPlayerRef _returnvalue))

(event EventTick
  (params (DeltaSeconds :type Float%20%28single-precision%29))
  (bind _audio (Variables|Default|GetAudio))
  ;[1 1 1] Finished lockpick
  (Utilities|FlowControl|Sequence
    (:then_0
      (if (Variables|/Game/BP_Actors/Player.Player_C|GetInPuzzelTrigger (Variables|Default|GetPlayerRef))
        (Utilities|FlowControl|DoOnce false :!label _label
          (:Completed
            (Audio|Components|Audio|Stop _audio)
            (goto _label_2 Reset)))
        (else
          (Utilities|FlowControl|DoOnce false :!label _label_2
            (:Completed
              (Audio|Components|Audio|Play _audio 0.0)
              (goto _label Reset))))))
    (:then_1
      (if (== (Variables|Default|GetMax) -1)
        (Audio|PlaySound2D "/Game/Audio/Cues/DoorOpen_Cue.DoorOpen_Cue" 1.0 1.0 0.0 0 0)
        (Default|CallLockComplete)
        (CallFunction|ResetLock)
        (bind _returnvalue (Actor|GetActorOfClass "/Game/BP_Actors/Player.Player_C"))
        (Default|LockPickComplete _returnvalue)
        (Default|CallOnToggleWolfHowl _returnvalue true)))))

(event EventInteract
  (bind _dor (Variables|Default|Getdor))
  ;[1 1 1] interface function
  (Transformation|SetWorldLocation _dor (Math|Vector|MakeVector 0.0 0.0 (- (.z (Transformation|GetWorldLocation _dor)) 5e+02)) false false)
  (Utilities|FlowControl|Delay 0.2)
  (Actor|DestroyActor))

(fn ConstructionScript)

(fn RemovesElementfromArrayifItExists
  (for _array_element (Variables|Default|GetNotCompletedLocks)
    (if (Utilities|Enum|Equal(Enum) _array_element (Variables|Default|GetCurrentLockEnum))
      (Utilities|Array|RemoveItem (Variables|Default|GetNotCompletedLocks) (Variables|Default|GetCurrentLockEnum))
      (Audio|PlaySound2D "/Game/Audio/Cues/LockPickLåsIn_Cue.LockPickLåsIn_Cue" 1.0 1.0 0.0 0 0)
      (Variables|Default|SetMax (- (Variables|Default|GetMax) 1))
      (CallFunction|SetCounter))))

(fn ResetLock
  (Variables|Default|SetNotCompletedLocks (Variables|Default|GetNotCompletedLocks_Copy))
  (Variables|Default|SetMax 2))