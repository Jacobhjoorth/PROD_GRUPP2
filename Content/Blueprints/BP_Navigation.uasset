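; BP_Navigation is a trigger that halts the player and hands them a Direction, apparently at a navigation choice point.
; On its first collision overlap, a player-tagged actor makes it fetch the Player, rotate it 180 degrees if AxisValue is negative, pass Direction to OnTriggerOverlap and disable movement.
; During the intro it also plays the narrator's right-or-left line.
; A DoOnce guard precedes the tag check, so any first overlap consumes the trigger.
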(event OnComponentBeginOverlap(Collision)
  (params (OverlappedComponent :type Primitive%20Component%20Object%20Reference) (OtherActor :type Actor%20Object%20Reference) (OtherComp :type Primitive%20Component%20Object%20Reference) (OtherBodyIndex :type Integer) (bFromSweep :type Boolean) (SweepResult :type Hit%20Result%20Structure%20%28by%20ref%29))
  (Utilities|FlowControl|DoOnce false
    (:Completed
      (if (Actor|ActorHasTag OtherActor "player")
        (bind _returnvalue (Actor|GetActorOfClass "/Game/BP_Actors/Player.Player_C"))
        (if (< (Variables|/Game/BP_Actors/Player.Player_C|GetAxisValue _returnvalue) 0.0)
          (Default|Rotate180 _returnvalue))
        (Default|OnTriggerOverlap _returnvalue (Variables|Default|GetDirection))
        (Pawn|Components|CharacterMovement|DisableMovement (Variables|/Script/Engine.Character|GetCharacterMovement _returnvalue))
        (if (Variables|/Game/BP_Actors/Player.Player_C|GetPlayerInIntro _returnvalue)
          (Audio|PlaySound2D "/Game/Audio/Intro/11NarratorRightOrLeft.11NarratorRightOrLeft" 1.0 1.0 0.0 0 0))))))

(event EventBeginPlay)

(event Collision|EventActorBeginOverlap
  (params (OtherActor :type Actor%20Object%20Reference)))

(event EventTick
  (params (DeltaSeconds :type Float%20%28single-precision%29)))

(fn ConstructionScript)