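; BPC_React is a component running a spacebar reaction quick-time event, triggered by enemy or object collisions, where failure kills the player.
; BeginReact plays tension audio, then opens the press window after a delay.
; A looping timer drives ReactTick, which polls Space and fails early presses or, via retriggerable delay, missed ones.
; Successes repeat the round with higher-pitched sounds until TotalReacts is reached, then OnStopReact fires.
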(event Custom|Begin%20React
  (bind _react_start_sfx (Variables|Default|GetReact_Start_SFX))
  ;[0.05729 0.05729 0.05729] Beginplay, enables space press after delay (delay is 0 for now), then another delay for the player to press space to react
  (CallFunction|ReactTick)
  (Variables|Default|SetIs%20Reacting true)
  (bind _pitch_multiplier (CallFunction|IncreasePitch 0.1055))
  (Variables|/Script/Engine.AudioComponent|SetPitchMultiplier _react_start_sfx (- _pitch_multiplier 0.14))
  (Audio|Components|Audio|Stop _react_start_sfx)
  (Audio|Components|Audio|Play _react_start_sfx 0.0)
  (Development|PrintString "Dont press space yet")
  (Audio|Components|Audio|Play (Variables|Default|GetReact_Tension_SFX) 0.0)
  (Utilities|FlowControl|Delay 1.7) ; delay b4 player should press space
  (if (Variables|Default|GetIs%20Reacting)
    (Variables|Default|SetShould%20Press%20Spacebar true)
    (Development|PrintString "press space to react")
    (Audio|Components|Audio|Play (Variables|Default|GetReact_ToReact_SFX) 0.0)))

(event Custom|React%20Tick
  (bind _react_success_sfx (Variables|Default|GetReact_Success_SFX))
  (bind _react_counter_checker (Variables|Default|GetReact%20Counter%20Checker))
  ;[0.05729 0.05729 0.05729] Checks if player pressed space after space has been enabled
  (bind _returnvalue (Utilities|Time|SetTimerbyEvent (delegate Custom|React%20Tick) 0.01 true))
  (Variables|Default|SetTimer%20Handle _returnvalue)
  (if (Variables|Default|GetCan%20Press%20Space)
    (if (Variables|Default|GetShould%20Press%20Spacebar)
      (if (Game|Player|IsInputKeyDown (Game|GetPlayerController 0) "SpaceBar")
        ;[0.05729 0.05729 0.05729] React success
        (Variables|Default|SetShould%20Press%20Spacebar false)
        (Utilities|Time|ClearandInvalidateTimerbyHandle (Variables|Default|GetTimer%20Handle))
        (Development|PrintString "spacebar successfully pressed")
        (Audio|Components|Audio|Stop (Variables|Default|GetReact_Tension_SFX))
        (bind _pitch_multiplier (CallFunction|IncreasePitch 0.15))
        (Variables|/Script/Engine.AudioComponent|SetPitchMultiplier _react_success_sfx _pitch_multiplier)
        (Audio|Components|Audio|Stop _react_success_sfx)
        (Audio|Components|Audio|Play _react_success_sfx 0.0)
        ;[0.05729 0.05729 0.05729] Calculates how many times to react
        (bind _result (Math|Integer|IncrementInt (Variables|Default|GetReact%20Counter))
          (:%20%20
            (if (== _result (Variables|Default|GetTotal%20Reacts))
              ;[0.05729 0.05729 0.05729] React finished
              (Development|PrintString "react successfull")
              (Utilities|Time|ClearandInvalidateTimerbyHandle (Variables|Default|GetTimer%20Handle))
              (Variables|Default|SetIs%20Reacting false)
              (Default|CallOnStopReact)
              (else
                ;[0.05729 0.05729 0.05729] React not finished and resets
                (Utilities|FlowControl|Delay (Variables|Default|GetTime%20To%20React))
                (CallFunction|RestartReact))))))
      (else
        (Utilities|FlowControl|Sequence
          (:then_0
            (Utilities|FlowControl|RetriggerableDelay (Variables|Default|GetTime%20To%20React))
            ;[0.05729 0.05729 0.05729] Failchecks
            (if (<= (Variables|Default|GetReact%20Counter) _react_counter_checker)
              (Development|PrintString "spacebar failed to press")
              ;[0.05729 0.05729 0.05729] React failed
              (if (Variables|Default|GetIs%20Reacting) :!label _label
                (Utilities|Time|ClearandInvalidateTimerbyHandle (Variables|Default|GetTimer%20Handle))
                (Development|PrintString " failed react")
                (|CancelSounds)
                (Variables|Default|SetIs%20Reacting false)
                (Default|CallOnStopReact self)
                (Default|PlayerDeath (Variables|Default|GetPlayer)))
              (else
                (Math|Integer|IncrementInt _react_counter_checker))))
          (:then_1
            (if (Game|Player|IsInputKeyDown (Game|GetPlayerController 0) "SpaceBar")
              (Development|PrintString "spacebar pressed too quick")
              (goto _label))))))))

(event Custom|StartReactEnemy
  ;[0.05729 0.05729 0.05729] Start react on enemy collision with player
  (Utilities|StartReactEvents)
  (Default|CallOnStartReactEnemy self))

(event Custom|StartReactObject
  ;[0.05729 0.05729 0.05729] Start react on object collision with player
  (Utilities|StartReactEvents))

(event EventBeginPlay
  (bind _self self)
  (|CreateSound)
  (EventDispatchers|BindEventtoOnStartReactEnemy _self (EventDispatchers|CreateEvent :!event Custom|StartReactEnemy))
  (EventDispatchers|BindEventtoOnStartReactObject _self (EventDispatchers|CreateEvent :!event Custom|StartReactObject)))

(fn IncreasePitch
  (params (Multiply :type Float%20%28double-precision%29))
  (return (+ (* (Math|Conversions|ToFloat(Integer) (Variables|Default|GetReact%20Counter)) Multiply) 1.0)))

(fn RestartReact
  (CallFunction|BeginReact)
  (Variables|Default|SetShould%20Press%20Spacebar false))