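; Trigger box that halts the player and presents a set of available options, apparently direction choices.
; When an actor tagged "player" enters the box, it finds the Player actor by class, passes AvailableOptions to OnTriggerOverlap and disables character movement.
; A MovePlayer event receives the picked Direction but only prints it; nothing here moves the player or re-enables movement.
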(event OnComponentBeginOverlap(Box)
  (params (OverlappedComponent :type Primitive%20Component%20Object%20Reference) (OtherActor :type Actor%20Object%20Reference) (OtherComp :type Primitive%20Component%20Object%20Reference) (OtherBodyIndex :type Integer) (bFromSweep :type Boolean) (SweepResult :type Hit%20Result%20Structure%20%28by%20ref%29))
  (if (Actor|ActorHasTag OtherActor "player")
    (bind _returnvalue (Actor|GetActorOfClass "/Game/BP_Actors/Player.Player_C"))
    (Default|OnTriggerOverlap _returnvalue (Variables|Default|GetAvailable%20Options))
    (Pawn|Components|CharacterMovement|DisableMovement (Variables|/Script/Engine.Character|GetCharacterMovement _returnvalue))))

(event Custom|MovePlayer_1
  (params (Direction :type ENUM_Directions%20Enum :default "NewEnumerator0"))
  (Development|PrintString "The player picked: ")
  (Development|PrintString (Utilities|String|EnumtoString Direction)))

(event EventBeginPlay)

(event EventTick
  (params (DeltaSeconds :type Float%20%28single-precision%29)))

(fn ConstructionScript)