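; BP_TunePuzzle is a prototype tune puzzle in which the player repeats a fixed four-tone sequence.
; StartPuzzle sets the sequence, and Space prints CurrentToneIndex at timed intervals as stand-in playback.
; Four press events append their tone and compare arrays to set PuzzleSolved, though only the first calls CallTuneComplete.
; Length checking, input clearing and replay on failure exist only as placeholder debug prints, partly in Swedish.
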(event Custom|PlayCorrectSequence
  (for _array_element (Variables|Default|GetCorrectToneSequence)
    (Development|PrintString (Utilities|String|ToString(Integer) (Variables|Default|GetCurrentToneIndex)))
    (Utilities|FlowControl|Delay 0.5)))

(event Custom|PlayerPress1
  (Utilities|Array|Add (Variables|Default|GetPlayerToneSequence) 1)
  (Development|PrintString "Kolla Om PlayerToneSequence innehåller 4 saker i arreyen")
  (if (Utilities|Array|Identical (Variables|Default|GetCorrectToneSequence) (Variables|Default|GetPlayerToneSequence))
    (Variables|Default|SetbPuzzleSolved true)
    (Default|CallTuneComplete)
    (else
      (Development|PrintString "Clear playerToneSquence"))))

(event Custom|PlayerPress2
  (Utilities|Array|Add (Variables|Default|GetPlayerToneSequence) 2)
  (Development|PrintString "Kolla Om PlayerToneSequence innehåller 4 saker i arreyen")
  (if (Utilities|Array|Identical (Variables|Default|GetCorrectToneSequence) (Variables|Default|GetPlayerToneSequence))
    (Variables|Default|SetbPuzzleSolved true)
    (else
      (Development|PrintString "Clear playerToneSquence"))))

(event Custom|PlayerPress3
  (Utilities|Array|Add (Variables|Default|GetPlayerToneSequence) 3)
  (Development|PrintString "Kolla Om PlayerToneSequence innehåller 4 saker i arreyen")
  (if (Utilities|Array|Identical (Variables|Default|GetCorrectToneSequence) (Variables|Default|GetPlayerToneSequence))
    (Variables|Default|SetbPuzzleSolved true)
    (else
      (Development|PrintString "Clear playerToneSquence"))))

(event Custom|PlayerPress4
  (Utilities|Array|Add (Variables|Default|GetPlayerToneSequence) 4)
  (Development|PrintString "Kolla Om PlayerToneSequence innehåller 4 saker i arreyen")
  (if (Utilities|Array|Identical (Variables|Default|GetCorrectToneSequence) (Variables|Default|GetPlayerToneSequence))
    (Variables|Default|SetbPuzzleSolved true)
    (else
      (Development|PrintString "Clear playerToneSquence")
      (Development|PrintString "Spela upp CorrectToneSequence igen"))))

(event EventStartPuzzle
  (Variables|Default|SetCorrectToneSequence (Utilities|Array|MakeArray 1 2 3 4))
  (Development|PrintString "Melodi spelar med följden: 1-2-3-4" true true "(R=0.000000,G=0.660000,B=1.000000,A=1.000000)" 1e+01))

(event Input|KeyboardEvents|SpaceBar
  (params (Key :type Key%20Structure :default "None"))
  (:Pressed
    (CallFunction|PlayCorrectSequence)))

(fn ConstructionScript
  (|CallParentFunction))