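; Scripts the intro level: a voiced dialogue with Mike and narrator tutorial prompts, plus an event that opens Main.
; Audio components chain through OnAudioFinished, with input enabled after the opening lines and a looping timer polling for forward input.
; A counter indexes Mike's clip array so Tick keeps the current clip beside the player for the first eight entries.
; Mid-sequence the player is teleported, and a trigger box later freezes movement to start the walkie-talkie exchange.
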(event OnAudioFinished(Areyouokay?)
  ;[1 1 1] Yeah, im fine.
  (Utilities|FlowControl|Delay 0.5)
  (Audio|Components|Audio|Play (Variables|Default|GetYeah%20im%20fine) 0.0)
  (bind _result (Math|Integer|IncrementInt (Variables|Default|GetCurrentAudioCounter))
    (:%20%20
      (bind _output_get (Variables|Default|SetCurrentAudioCounter _result))
      (Development|PrintString (Utilities|String|ToString(Integer) _output_get)))))

(event OnAudioFinished(Yeahimfine)
  ;[1 1 1] Come on were almost there!
  (Audio|Components|Audio|Play (Variables|Default|GetComeOnWere) 0.0))

(event OnAudioFinished(8MikeAreYouSerious)
  ;[1 1 1] We'll be fine
  (Audio|Components|Audio|Play (Variables|Default|Get9WellBeFine) 0.0))

(event OnAudioFinished(9WellBeFine)
  ;[1 1 1] Take a left here!
  (Audio|Components|Audio|Play (Variables|Default|Get10TakeALeft) 0.0)
  (bind _result (Math|Integer|IncrementInt (Variables|Default|GetCurrentAudioCounter))
    (:%20%20
      (bind _output_get (Variables|Default|SetCurrentAudioCounter _result))
      (Development|PrintString (Utilities|String|ToString(Integer) _output_get))
      (Utilities|FlowControl|Delay 2.0)
      (Transformation|SetActorLocation (Variables|Default|GetPlayer) "4420.000000,5060.000000,0.000000" false false))))

(event OnAudioFinished(10TakeALeft)
  ;[1 1 1] Narrator Left or right
  (bind _result (Math|Integer|IncrementInt (Variables|Default|GetCurrentAudioCounter))
    (:%20%20
      (bind _output_get (Variables|Default|SetCurrentAudioCounter _result))
      (Development|PrintString (Utilities|String|ToString(Integer) _output_get)))))

(event OnAudioFinished(12AhThereItIs)
  ;[1 1 1] Thats scary!
  (Audio|Components|Audio|Play (Variables|Default|Get13ThatsScary) 0.0)
  (bind _result (Math|Integer|IncrementInt (Variables|Default|GetCurrentAudioCounter))
    (:%20%20
      (bind _output_get (Variables|Default|SetCurrentAudioCounter _result))
      (Development|PrintString (Utilities|String|ToString(Integer) _output_get)))))

(event OnAudioFinished(13ThatsScary)
  ;[1 1 1] Here take this walkie talkie
  (Utilities|FlowControl|Delay 1.0)
  (Audio|Components|Audio|Play (Variables|Default|Get14HereTakeThisWalkieTalkie) 0.0))

(event OnAudioFinished(14HereTakeThisWalkieTalkie)
  ;[1 1 1] Thanks..
  (Audio|Components|Audio|Play (Variables|Default|Get15OhThanks) 0.0)
  (bind _result (Math|Integer|IncrementInt (Variables|Default|GetCurrentAudioCounter))
    (:%20%20
      (bind _output_get (Variables|Default|SetCurrentAudioCounter _result))
      (Development|PrintString (Utilities|String|ToString(Integer) _output_get)))))

(event OnAudioFinished(15OhThanks)
  ;[1 1 1] Yeah no prob
  (Audio|Components|Audio|Play (Variables|Default|Get16YeahNoProbComeHelpMeGetThisDoor) 0.0))

(event OnAudioFinished(16YeahNoProbComeHelpMeGetThisDoor)
  (Audio|Components|Audio|Play (Variables|Default|Get17NarratorInteract) 0.0))

(event OnAudioFinished(7TheFeelingThatSmthTerrible)
  ;[1 1 1] Mike are you serious
  (Audio|Components|Audio|Play (Variables|Default|Get8MikeAreYouSerious) 0.0)
  (bind _result (Math|Integer|IncrementInt (Variables|Default|GetCurrentAudioCounter))
    (:%20%20
      (bind _output_get (Variables|Default|SetCurrentAudioCounter _result))
      (Development|PrintString (Utilities|String|ToString(Integer) _output_get)))))

(event OnAudioFinished(ComeOnWere)
  ;[1 1 1] Narrator, Press W to move forward
  (Audio|Components|Audio|Play (Variables|Default|GetNarratorPressW) 0.0)
  (Input|EnableInput (Variables|Default|GetPlayer) 0)
  (bind _result (Math|Integer|IncrementInt (Variables|Default|GetCurrentAudioCounter))
    (:%20%20
      (bind _output_get (Variables|Default|SetCurrentAudioCounter _result))
      (Development|PrintString (Utilities|String|ToString(Integer) _output_get)))))

(event OnComponentBeginOverlap(Navigationtriggerbox)
  (params (OverlappedComponent :type Primitive%20Component%20Object%20Reference) (OtherActor :type Actor%20Object%20Reference) (OtherComp :type Primitive%20Component%20Object%20Reference) (OtherBodyIndex :type Integer) (bFromSweep :type Boolean) (SweepResult :type Hit%20Result%20Structure%20%28by%20ref%29))
  ;[1 1 1] There it is!
  (if (Actor|ActorHasTag OtherActor "player")
    (Utilities|FlowControl|DoOnce false
      (:Completed
        (Pawn|Components|CharacterMovement|DisableMovement (Variables|/Script/Engine.Character|GetCharacterMovement (Variables|Default|GetPlayer)))
        (Audio|Components|Audio|Play (Variables|Default|Get12AhThereItIs) 0.0)
        (Audio|Components|Audio|Play (Variables|Default|GetSpookySound) 0.0)))))

(event OnAudioFinished(NarratorPressW)
  (CallFunction|CheckNarratorPressW))

(event OnAudioFinished(Doyoufeelit?)
  ;[1 1 1] Feel what?
  (Audio|Components|Audio|Play (Variables|Default|GetFeel%20What?) 0.0)
  (bind _result (Math|Integer|IncrementInt (Variables|Default|GetCurrentAudioCounter))
    (:%20%20
      (bind _output_get (Variables|Default|SetCurrentAudioCounter _result))
      (Development|PrintString (Utilities|String|ToString(Integer) _output_get)))))

(event OnAudioFinished(FeelWhat?)
  ;[1 1 1] That feeling that smth
  (Audio|Components|Audio|Play (Variables|Default|Get7TheFeelingThatSmthTerrible) 0.0))

(event Custom|Load%20next%20level
  ;[1 1 1] Load next level
  (Variables|/Game/BP_Actors/Player.Player_C|SetPlayerInIntro (Variables|Default|GetPlayer) false)
  (Development|PrintString "TRIED TO LOAD NEXT LEVEL")
  (Utilities|FlowControl|Delay 0.2)
  (Development|PrintString "NEW LEVEL LOADED")
  (Game|OpenLevel(byName) "Main"))

(event Custom|TurnLeft
  (Audio|PlaySound2D "/Game/Audio/Sounds/Voices/PerfectYouHaveNowTurnedLeft.PerfectYouHaveNowTurnedLeft" 1.0 1.0 0.0 0 0))

(event Custom|CheckNarratorPressW
  (bind _returnvalue (Game|GetPlayerController 0))
  ;[1 1 1] Do you feel it?
  (bind _returnvalue_2 (Utilities|Time|SetTimerbyEvent (delegate Custom|CheckNarratorPressW) 0.01 true))
  (if (or (Game|Player|IsInputKeyDown _returnvalue "W") (Game|Player|IsInputKeyDown _returnvalue "Up"))
    (Utilities|Time|ClearandInvalidateTimerbyHandle _returnvalue_2)
    (Audio|Components|Audio|Play (Variables|Default|GetDo%20you%20feel%20it?) 0.0)))

(event Custom|No%20Move%20Left%20Insted
  ;[1 1 1] You can't turn right
  (Utilities|FlowControl|DoOnce false :!label _label
    (:Completed
      (Audio|PlaySound2D "/Game/Audio/Sounds/Voices/NarratorNavigationLeftRightForward.NarratorNavigationLeftRightForward" 1.0 1.0 0.0 0 0)
      (Utilities|FlowControl|Delay 12.0)
      (goto _label Reset))))

(event Custom|Start%20First%20Sound
  ;[1 1 1] Are you alright?
  (Audio|Components|Audio|Play (Variables|Default|GetAre%20you%20okay?) 0.0))

(event EventBeginPlay
  (bind _13thatsscary (Variables|Default|Get13ThatsScary))
  ;[1 1 1] Beginplay, creat array, set bools
  (Variables|Default|SetAudio%20Array (Utilities|Array|MakeArray (Variables|Default|GetAre%20you%20okay?) (Variables|Default|GetComeOnWere) (Variables|Default|GetDo%20you%20feel%20it?) (Variables|Default|Get7TheFeelingThatSmthTerrible) (Variables|Default|Get9WellBeFine) (Variables|Default|Get10TakeALeft) (Variables|Default|Get12AhThereItIs) (Variables|Default|Get14HereTakeThisWalkieTalkie) (Variables|Default|Get16YeahNoProbComeHelpMeGetThisDoor) _13thatsscary (Variables|Default|Get15OhThanks) _13thatsscary _13thatsscary _13thatsscary))
  (bind _returnvalue (Actor|GetActorOfClass "/Game/BP_Actors/Player.Player_C"))
  (bind _output_get (Variables|Default|SetPlayer _returnvalue))
  (Variables|/Game/BP_Actors/Player.Player_C|SetPlayerInIntro _output_get true)
  (Variables|/Game/BP_Actors/Player.Player_C|SetCan%20Rotate _output_get false)
  (Input|DisableInput _returnvalue 0)
  (Utilities|FlowControl|Delay 2.0)
  (CallFunction|StartFirstSound))

(event EventTick
  (params (DeltaSeconds :type Float%20%28single-precision%29))
  (bind _currentaudiocounter (Variables|Default|GetCurrentAudioCounter))
  (if (< _currentaudiocounter 8)
    (Transformation|SetWorldLocation (Utilities|Array|Get(acopy) (Variables|Default|GetAudio%20Array) _currentaudiocounter) (+ (Transformation|GetActorLocation (Variables|Default|GetPlayer)) "150.000000,0.000000,0.000000") false false)))

(fn ConstructionScript)